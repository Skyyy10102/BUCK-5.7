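; Health component that tracks its owning actor's health, starting at max, and plays feedback for damage and healing.
; It binds to the owner's OnTakeAnyDamage, clamps health, fires OnTookDamage, and fires OnKilled when health is zero.
; Damage spawns sound, particles and a camera shake on player 0, whichever actor owns it.
; A healing event adds clamped health with sound and particles but is not bound here; Kill is an empty stub.
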(event `self.ReceiveBeginPlay`
  (set `self.Owner` (`self.GetOwner`))
  (set `self.Health` (`self.MaxHealth`))
  (add `Actor.OnTakeAnyDamage` (`self.Owner`) (`|CreateDelegate` :!event `TookDamage`)))

(event `TookDamage`
  (params (DamagedActor :type "Actor Object Reference") (Damage :type "Float (single-precision)") (DamageType :type "DamageType Object Reference") (InstigatedBy :type "Controller Object Reference") (DamageCauser :type "Actor Object Reference"))
  (set `self.Health` (`KismetMathLibrary.FClamp` (- (`self.Health`) Damage) 0.0 (`self.MaxHealth`)))
  (`self.PlayDamageFX`)
  (`self.OnTookDamage` Damage)
  (if (<= (`self.Health`) 0.0)
    (`self.OnKilled`)))

(event `TookHealing`
  (params (DamagedActor :type "Actor Object Reference") (Healing :type "Float (single-precision)") (DamageType :type "DamageType Object Reference") (InstigatedBy :type "Controller Object Reference") (DamageCauser :type "Actor Object Reference"))
  (set `self.Health` (`KismetMathLibrary.FClamp` (+ (`self.Health`) Healing) 0.0 (`self.MaxHealth`)))
  (`self.PlayHealFX`))

(fn `Kill`)

(fn `PlayDamageFX`
  (`GameplayStatics.PlaySoundAtLocation` (`self.DamageSound`) (`Actor.K2_GetActorLocation` (`self.Owner`)) (struct) 1.0 1.0 0.0 null null null null)
  (`NiagaraFunctionLibrary.SpawnSystemAtLocation` (`self.DamageParticles`) (`Actor.K2_GetActorLocation` (`self.Owner`)))
  (`LegacyCameraShake.StartLegacyCameraShake` (`GameplayStatics.GetPlayerCameraManager` 0) "/Script/EngineCameras.LegacyCameraShake" 999.0))

(fn `PlayHealFX`
  (`GameplayStatics.PlaySoundAtLocation` (`self.HealSound`) (`Actor.K2_GetActorLocation` (`self.Owner`)) (struct) 1.0 1.0 0.0 null null null null)
  (`NiagaraFunctionLibrary.SpawnSystemAtLocation` (`self.HealParticles`) (`Actor.K2_GetActorLocation` (`self.Owner`))))